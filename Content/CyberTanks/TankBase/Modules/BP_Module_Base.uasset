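; Base possessable tank module that players operate, forwarding Move and Interact input through dispatchers and returning them to their character on exit or vehicle destruction.
; ACEnergon tracks HP and energy; depletion marks the module broken and randomly picks a required part by failure type.
; An overlapping matching part restores it with invulnerability and is destroyed, while proximity shows the needed part in a popup.
; It also spawns random minigames for the controller.
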(event `self.ReceiveTick`
  (params (DeltaSeconds :type "Float (single-precision)"))
  (if (`|EnumEquality` (`self.UseState`) "NewEnumerator1")
    (`/Engine/EditorBlueprintResources/StandardMacros.DoOnce` false :!label _label
      (:`Completed`
        (`SceneComponent.SetVisibility` (`self.ExitToolTip`) false false)
        (goto _label_2 :!via `Reset`)))
    (else
      (`/Engine/EditorBlueprintResources/StandardMacros.DoOnce` false :!label _label_2
        (:`Completed`
          (`SceneComponent.SetVisibility` (`self.ExitToolTip`) true false)
          (goto _label :!via `Reset`))))))

(event `turnoffname`
  (`SceneComponent.SetVisibility` (`self.ModuleName`) false false))

(event `self.ReceiveBeginPlay`
  (`|ExecutionSequence`
    (:`then_0`
      (`self.InitPopUpWidget`))
    (:`then_1`
      (add `self.OnDestroyed` (`self.VehicleOwner`) (delegate `VehicleDestroyed`))
      (add `/Game/CyberTanks/EnergonComponent/AC_Energon.HPZero` (`self.AC_Energon`) (delegate `HPDroppedToZero`))
      (add `/Game/CyberTanks/EnergonComponent/AC_Energon.EnergyZero` (`self.AC_Energon`) (delegate `EnergyDroppedToZero`))
      (add `/Game/CyberTanks/EnergonComponent/AC_Energon.HPAndEnergyZero` (`self.AC_Energon`) (delegate `HPAndEnergyDroppedToZero`)))
    (:`then_2`
      (bind _aswbp_repair_pop_up (cast `/Game/CyberTanks/TankBase/Modules/WBP_RepairPopUp` (`WidgetComponent.GetWidget` (`self.ModuleName`))))
      (`/Game/CyberTanks/TankBase/Modules/WBP_RepairPopUp.ChangeTextTo` _aswbp_repair_pop_up (`KismetTextLibrary.Conv_StringToText` (`KismetSystemLibrary.GetObjectName` self)))
      (`KismetSystemLibrary.K2_SetTimerDelegate` (delegate `turnoffname`) 5.0))))

(event `HPDroppedToZero`
  (`KismetSystemLibrary.PrintString` "Hit Points 0")
  (`self.CheckEnergyAndHP`))

(event `EnergyDroppedToZero`
  (`KismetSystemLibrary.PrintString` "Energy 0" true true (struct :`R` 1.0 :`A` 1.0))
  (`self.CheckEnergyAndHP`))

(event `HPAndEnergyDroppedToZero`
  (`KismetSystemLibrary.PrintString` "HP and Energy 0")
  (`self.CheckEnergyAndHP`))

(event `VehicleDestroyed` :!signature `self.OnDestroyed`
  (params (DestroyedActor :type "Actor Object Reference"))
  (bind _aspc_mpgame (cast `/Game/CyberTanks/MultiPlayerSetup/PC_MPGame` (`self.GetController`))
    (:`then`
      (`/Game/CyberTanks/MultiPlayerSetup/PC_MPGame.SwitchToCharacter` _aspc_mpgame))
    (:`CastFailed`
      _))
  (`self.K2_DestroyActor`))

(event `EnhancedInput|/Game/ThirdPerson/Input/Actions/IA_Move`
  (params (ActionValue :type "Vector2D Structure") (ElapsedSeconds :type "Float (double-precision)") (TriggeredSeconds :type "Float (double-precision)") (InputAction :type "InputAction Object Reference" :default "/Game/ThirdPerson/Input/Actions/IA_Move.IA_Move"))
  (:`Triggered`
    (`self.MoveTriggeredEvent` ActionValue))
  (:`Started`
    (`self.MoveStartedEvent` ActionValue)))

(event `EnhancedInput|/Game/ThirdPerson/Input/Actions/IA_Interact`
  (params (ActionValue :type Boolean) (ElapsedSeconds :type "Float (double-precision)") (TriggeredSeconds :type "Float (double-precision)") (InputAction :type "InputAction Object Reference" :default "/Game/ThirdPerson/Input/Actions/IA_Interact.IA_Interact"))
  (:`Triggered`
    (`self.InteractTriggeredEvent`))
  (:`Started`
    (`self.InteractStartedEvent`)))

(event `EnhancedInput|/Game/ThirdPerson/Input/Actions/IA_Exit`
  (params (ActionValue :type Boolean) (ElapsedSeconds :type "Float (double-precision)") (TriggeredSeconds :type "Float (double-precision)") (InputAction :type "InputAction Object Reference" :default "/Game/ThirdPerson/Input/Actions/IA_Exit.IA_Exit"))
  (:`Started`
    (bind _aspc_mpgame (cast `/Game/CyberTanks/MultiPlayerSetup/PC_MPGame` (`self.GetController`)))
    (`/Game/CyberTanks/MultiPlayerSetup/PC_MPGame.SwitchToCharacter` _aspc_mpgame)))

(event `self.ReceivePossessed`
  (params (NewController :type "Controller Object Reference"))
  ; Check if char has whats needed for repair
  (cast `/Game/CyberTanks/MultiPlayerSetup/PC_MPGame` NewController)
  (`self.CheckEnergyAndHP`))

(event `StartMiniGameEvent`
  (params (ReasonForMiniGame :type "/Game/CyberTanks/MiniGame/ENUM_WhyMiniGameStarted Enum" :default "NewEnumerator0"))
  ;[0.15 0.04419 0 0.5] Change to Maintanance need Legacy, send to move this to PartFabricator
  (bind _aspc_mpgame (cast `/Game/CyberTanks/MultiPlayerSetup/PC_MPGame` (`self.GetController`))
    (:`then`
      (bind _returnvalue (`|SpawnActorFromClass` (`KismetArrayLibrary.Array_Random` (`|MakeArray` "/Game/CyberTanks/MiniGame/MoroGame/BP_MiniGame_Moro.BP_MiniGame_Moro_C" "/Game/CyberTanks/MiniGame/MinigameMoro2/BP_MiniGame_Moro_2.BP_MiniGame_Moro_2_C" "/Game/CyberTanks/MiniGame/MoroGame3/BP_MiniGame_Moro_3.BP_MiniGame_Moro_3_C" :!type "Actor Class Reference")) (`self.MiniGameSpawnTransform`) "AdjustIfPossibleButAlwaysSpawn" "MultiplyWithRoot" null null))
      (bind _asbp_mini_game_base (cast `/Game/CyberTanks/MiniGame/BP_MiniGame_Base` _returnvalue)
        (:`then`
          (`/Game/CyberTanks/MultiPlayerSetup/PC_MPGame.SwitchToMiniGame` _aspc_mpgame _asbp_mini_game_base self ReasonForMiniGame))
        (:`CastFailed`
          (`KismetSystemLibrary.PrintString` "minigierka error"))))
    (:`CastFailed`
      (`KismetSystemLibrary.PrintString` "huge error"))))

(event `CheckEnergyAndHP`
  ; Create Maintanance need, and display
  (if (`self.Broken`)
    (`KismetSystemLibrary.PrintString` "cant use needs repair")
    (`KismetSystemLibrary.DelayUntilNextTick`)
    (`KismetSystemLibrary.DelayUntilNextTick`)
    (`KismetSystemLibrary.DelayUntilNextTick`)
    (bind _aspc_mpgame (cast `/Game/CyberTanks/MultiPlayerSetup/PC_MPGame` (`self.GetController`)))
    (`/Game/CyberTanks/MultiPlayerSetup/PC_MPGame.SwitchToCharacter` _aspc_mpgame)
    (else
      (bind _energonstate (`/Game/CyberTanks/EnergonComponent/AC_Energon.EnergonStateF` (`self.AC_Energon`)))
      (switch `/Game/CyberTanks/EnergonComponent/ENUM_EnergonState` _energonstate
        (:`NewEnumerator2`
          (set `self.HowToFix` "NewEnumerator2"))
        (:`NewEnumerator3`
          (set `self.HowToFix` "NewEnumerator1"))
        (:`NewEnumerator4`
          (set `self.HowToFix` "NewEnumerator3")))
      (set `self.Broken` true)
      (`KismetSystemLibrary.PrintString` "cant use needs repair")
      (`self.RandomizeWithWhatToFix`))))

(event `RandomizeWithWhatToFix`
  (switch `/Game/CyberTanks/MiniGame/ENUM_WhyMiniGameStarted` (`self.HowToFix`)
    (:`NewEnumerator1`
      (set `self.WithWhatToFix` (`KismetArrayLibrary.Array_Random` (`|MakeArray` "NewEnumerator0" "NewEnumerator1" :!type "/Game/CyberTanks/TankBase/Modules/PartsFabricator/ENUM_RepairNeed Enum"))))
    (:`NewEnumerator2`
      (set `self.WithWhatToFix` (`KismetArrayLibrary.Array_Random` (`|MakeArray` "NewEnumerator2" "NewEnumerator1" :!type "/Game/CyberTanks/TankBase/Modules/PartsFabricator/ENUM_RepairNeed Enum"))))
    (:`NewEnumerator3`
      (set `self.WithWhatToFix` (`KismetArrayLibrary.Array_Random` (`|MakeArray` "NewEnumerator0" "NewEnumerator1" "NewEnumerator2" :!type "/Game/CyberTanks/TankBase/Modules/PartsFabricator/ENUM_RepairNeed Enum"))))))

(event `Repair`
  (params (`PartCarried?` :type Boolean))
  (bind _ac_energon (`self.AC_Energon`))
  (set `self.Broken` false)
  (switch `/Game/CyberTanks/MiniGame/ENUM_WhyMiniGameStarted` (`self.HowToFix`)
    (:`NewEnumerator1`
      (`/Game/CyberTanks/EnergonComponent/AC_Energon.FullRestoreEnergy` _ac_energon true `PartCarried?`))
    (:`NewEnumerator2`
      (`/Game/CyberTanks/EnergonComponent/AC_Energon.FullRestoreHp` _ac_energon true `PartCarried?`))
    (:`NewEnumerator3`
      (`/Game/CyberTanks/EnergonComponent/AC_Energon.FullRestore` _ac_energon true `PartCarried?`))))

(event `self.CollisionToCheckPart.OnComponentBeginOverlap`
  (params (OverlappedComponent :type "PrimitiveComponent Object Reference") (OtherActor :type "Actor Object Reference") (OtherComp :type "PrimitiveComponent Object Reference") (OtherBodyIndex :type Integer) (bFromSweep :type Boolean) (SweepResult :type "HitResult Structure (by ref)"))
  ; Kickable part repair logic
  (bind _canuse (`self.CanUse`))
  (if (not _canuse)
    (if (`KismetSystemLibrary.DoesImplementInterface` OtherActor "/Game/CyberTanks/TankBase/Modules/PartsFabricator/BPI_HasRepairPart.BPI_HasRepairPart_C")
      (bind (_repairneedpart _partcarried_) (message `/Game/CyberTanks/TankBase/Modules/PartsFabricator/BPI_HasRepairPart.WhatRepairPart` OtherActor))
      (if (`|EnumEquality` _repairneedpart (`self.WithWhatToFix`))
        (`KismetSystemLibrary.PrintString` "correct part")
        (`self.Repair` _partcarried_)
        (`KismetSystemLibrary.DelayUntilNextTick`)
        (`self.K2_DestroyActor` OtherActor)
        (`self.ClosePopUp`)
        (else
          (`KismetSystemLibrary.PrintString` (`KismetTextLibrary.Conv_TextToString` (`|FormatText` "wrong part, need:{a}" (`|GetEnumeratorNameAsString` (`self.WithWhatToFix`))))))))))

(event `/Game/CyberTanks/EnergonComponent/BPI_Energon.Damage`
  (params (HPDamage :type "Float (double-precision)") (EnergyDamage :type "Float (double-precision)"))
  (bind _ac_energon (`self.AC_Energon`))
  (if (`|EnumInequality` (`/Game/CyberTanks/EnergonComponent/AC_Energon.EnergonState` _ac_energon) "NewEnumerator0")
    (`/Game/CyberTanks/EnergonComponent/AC_Energon.Damage` _ac_energon HPDamage EnergyDamage)))

(event `InitPopUpWidget`
  (`SceneComponent.SetVisibility` (`self.RepairPopUp`) false false)
  (add `/Game/CyberTanks/EnergonComponent/AC_Energon.HpOrEnergyChanged` (`self.AC_Energon`) (`|CreateDelegate` :!event `UpdateBars`)))

(event `ShowPopUp`
  (bind _aswbp_repair_pop_up (cast `/Game/CyberTanks/TankBase/Modules/WBP_RepairPopUp` (`WidgetComponent.GetWidget` (`self.RepairPopUp`)))
    (:`then`
      (if (`self.Broken`)
        (`/Game/CyberTanks/TankBase/Modules/WBP_RepairPopUp.ChangeTextTo` _aswbp_repair_pop_up (`|GenericToText` (`|GetEnumeratorNameAsString` (`self.WithWhatToFix`))))
        (`SceneComponent.SetVisibility` (`self.RepairPopUp`) true false)))
    (:`CastFailed`
      (`KismetSystemLibrary.PrintString` "in module cast to wbprepairpopup failed" true true (struct :`R` 1.0 :`G` 0.038133 :`A` 1.0)))))

(event `ClosePopUp`
  (`SceneComponent.SetVisibility` (`self.RepairPopUp`) false false))

(event `self.SphereCollisionPopUp.OnComponentBeginOverlap`
  (params (OverlappedComponent :type "PrimitiveComponent Object Reference") (OtherActor :type "Actor Object Reference") (OtherComp :type "PrimitiveComponent Object Reference") (OtherBodyIndex :type Integer) (bFromSweep :type Boolean) (SweepResult :type "HitResult Structure (by ref)"))
  (cast `/Game/ThirdPerson/Blueprints/BP_ThirdPersonCharacter` OtherActor)
  (`self.ShowPopUp`))

(event `self.SphereCollisionPopUp.OnComponentEndOverlap`
  (params (OverlappedComponent :type "PrimitiveComponent Object Reference") (OtherActor :type "Actor Object Reference") (OtherComp :type "PrimitiveComponent Object Reference") (OtherBodyIndex :type Integer))
  (cast `/Game/ThirdPerson/Blueprints/BP_ThirdPersonCharacter` OtherActor)
  (`self.ClosePopUp`))

(event `UpdateBars`
  (bind _ac_energon (`self.AC_Energon`))
  (bind _aswbp_energon_status (cast `/Game/CyberTanks/TankBase/Modules/WBP_EnergonStatus` (`WidgetComponent.GetWidget` (`self.Indicator`))))
  (`/Game/CyberTanks/TankBase/Modules/WBP_EnergonStatus.UpdateBars` _aswbp_energon_status (`/Game/CyberTanks/EnergonComponent/AC_Energon.HP` _ac_energon) (`/Game/CyberTanks/EnergonComponent/AC_Energon.MaxHp` _ac_energon) (`/Game/CyberTanks/EnergonComponent/AC_Energon.Energy` _ac_energon) (`/Game/CyberTanks/EnergonComponent/AC_Energon.MaxEnergy` _ac_energon)))

(fn `CanUse`
  (returns (CanUse :type Boolean))
  (return (or (`|EnumEquality` (`/Game/CyberTanks/EnergonComponent/AC_Energon.EnergonState` (`self.AC_Energon`)) "NewEnumerator0") (`|EnumEquality` (`/Game/CyberTanks/EnergonComponent/AC_Energon.EnergonState` (`self.AC_Energon`)) "NewEnumerator1"))))

(fn `UserConstructionScript`)