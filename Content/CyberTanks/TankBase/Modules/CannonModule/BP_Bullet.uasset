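; Cannon projectile for CyberTanks that can home in on enemies and explodes for area HP and energy damage.
; On BeginPlay it sets its speed and, if owned by a tank part, sphere-sweeps ahead and homes on the first melee or moving enemy found.
; Its Hit event sphere-traces the blast radius, damages each unique BPI_Energon actor, then destroys the bullet.
; The explosion trace still draws debug shapes.
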(event `self.ReceiveBeginPlay`
  (bind _projectilemovement (`self.ProjectileMovement`))
  (bind _bulletspeed (`self.BulletSpeed`))
  (set `ProjectileMovementComponent.InitialSpeed` _bulletspeed _projectilemovement)
  (set `ProjectileMovementComponent.MaxSpeed` _bulletspeed _projectilemovement)
  (set `MovementComponent.Velocity` (* (`self.GetActorForwardVector` self) _bulletspeed) _projectilemovement)
  (set `ProjectileMovementComponent.HomingAccelerationMagnitude` (`self.HomingAcceleration`) _projectilemovement)
  (`self.TraceEnemies`))

(event `self.ProjectileMovement.OnProjectileBounce`
  (params (ImpactResult :type "HitResult Structure (by ref)") (ImpactVelocity :type "Vector Structure (by ref)")))

(event `self.ReceiveHit`
  (params (MyComp :type "PrimitiveComponent Object Reference") (Other :type "Actor Object Reference") (OtherComp :type "PrimitiveComponent Object Reference") (bSelfMoved :type Boolean) (HitLocation :type "Vector Structure") (HitNormal :type "Vector Structure") (NormalImpulse :type "Vector Structure") (Hit :type "HitResult Structure (by ref)"))
  (`self.BulletExplosion` (`.Location` (`GameplayStatics.BreakHitResult` Hit)) (`self.ExplosionRadius`))
  (`self.K2_DestroyActor`))

(event `BulletExplosion`
  (params (Position :type "Vector Structure") (RadiusOfExplosion :type "Float (single-precision)"))
  (bind _outhits (`KismetSystemLibrary.SphereTraceMulti` :`Start` Position :`End` Position :`Radius` RadiusOfExplosion :`TraceChannel` "TraceTypeQuery1" :`DrawDebugType` "ForDuration"))
  (`KismetArrayLibrary.Array_Clear` (`self.ActorsToDamage`))
  (for _array_element _outhits
    (bind (_bblockinghit _binitialoverlap _time _distance _location _impactpoint _normal _impactnormal _physmat _hitactor) (`GameplayStatics.BreakHitResult` _array_element))
    (if (`KismetSystemLibrary.DoesImplementInterface` _hitactor "/Game/CyberTanks/EnergonComponent/BPI_Energon.BPI_Energon_C")
      (bind _asbpi_energon (cast `/Game/CyberTanks/EnergonComponent/BPI_Energon` _hitactor))
      (`KismetArrayLibrary.Array_AddUnique` (`self.ActorsToDamage`) _asbpi_energon)))
  (`/Game/CyberTanks/EnergonComponent/BPI_Energon.Damage` (`self.ActorsToDamage`) (`self.HPDamage`) (`self.EnergyDamage`)))

(event `TraceEnemies`
  (bind _returnvalue (`SceneComponent.K2_GetComponentLocation` (`self.BulletMesh`)))
  (`KismetSystemLibrary.IsObjectOfSoftClass` (`self.GetOwner`) "/Game/CyberTanks/TankBase/Modules/BP_TankPart_Base.BP_TankPart_Base_C"
    (:`True`
      (bind _outhits (`KismetSystemLibrary.SphereTraceMultiForObjects` _returnvalue (+ _returnvalue (* (`self.GetActorForwardVector`) (`self.HomingSearchDistance`))) (`self.HomingSearchRadius`) (`|MakeArray` "ObjectTypeQuery3" :!type "EObjectTypeQuery Enum")))
      (for _array_element _outhits
        (bind (_bblockinghit _binitialoverlap _time _distance _location _impactpoint _normal _impactnormal _physmat _hitactor _hitcomponent) (`GameplayStatics.BreakHitResult` _array_element))
        (`KismetSystemLibrary.IsObjectOfSoftClass` _hitactor "/Game/CyberTanks/Enemies/EnemyBases/Melee/BP_Enemy_Melee_Base.BP_Enemy_Melee_Base_C"
          (:`True`
            _)
          (:`False`
            (`KismetSystemLibrary.IsObjectOfSoftClass` _hitactor "/Game/CyberTanks/Enemies/EnemyBases/Ranged/BP_Enemy_Moving_Base.BP_Enemy_Moving_Base_C"
              (:`True`
                _))))
        (set `ProjectileMovementComponent.HomingTargetComponent` _hitcomponent (`self.ProjectileMovement`))
        (set `ProjectileMovementComponent.bIsHomingProjectile` true (`self.ProjectileMovement`))
        (break)))))

(fn `UserConstructionScript`)