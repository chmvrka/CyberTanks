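; Tank module in CyberTanks that fabricates a repair part after a production delay, starting with a default type on BeginPlay.
; OpenChooseMenu shows a WBP_PartFabricator widget linked to this fabricator, and ChoosePart stores the type and starts a looping countdown timer.
; At zero the timer clears and CreatePart spawns one BP_RepairPart at PartsSpawnLocation, named after the chosen type and given a limited lifespan.
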(event `self.ReceiveBeginPlay`
  (`self.ChoosePart` "NewEnumerator2"))

(event `ChoosePart`
  (params (Repair :type "/Game/CyberTanks/TankBase/Modules/PartsFabricator/ENUM_RepairNeed Enum" :default "NewEnumerator0"))
  (set `self.Repair` Repair)
  (`self.StartTimerForPart` (`self.TimeToProduce`)))

(event `OpenChooseMenu`
  (params (OwningPlayer :type "PlayerController Object Reference"))
  ; Create widget
  (bind _returnvalue (`|CreateWidget` "/Game/CyberTanks/TankBase/Modules/PartsFabricator/WBP_PartFabricator.WBP_PartFabricator_C" OwningPlayer self))
  (`UserWidget.AddToViewport` _returnvalue 0))

(event `CreatePart`
  (bind _returnvalue (`|SpawnActorFromClass` "/Game/CyberTanks/TankBase/Modules/PartsFabricator/RepairPart/BP_RepairPart.BP_RepairPart_C" (`SceneComponent.K2_GetComponentToWorld` (`self.PartsSpawnLocation`)) "Undefined" "MultiplyWithRoot" null (`KismetStringLibrary.Conv_StringToName` (`|GetEnumeratorNameAsString` (`self.Repair`))) null))
  (`self.SetLifeSpan` _returnvalue (`self.PartLifeSpan`)))

(event `StartTimerForPart`
  (params (CountdownTime :type "Float (double-precision)"))
  ; Part creation timer
  (set `self.CountdownTime` CountdownTime)
  (bind _returnvalue (`KismetSystemLibrary.K2_SetTimerDelegate` (delegate `Countdown`) 0.1 true))
  (set `self.CountdownHandler` _returnvalue))

(event `Countdown`
  ; Part creation timer
  (bind _output_get (set `self.CountdownTime` (- (`self.CountdownTime`) 0.1)))
  (if (<= _output_get 0.0)
    (`KismetSystemLibrary.K2_ClearAndInvalidateTimerHandle` (`self.CountdownHandler`))
    (`self.CreatePart`)))

(fn `UserConstructionScript`)