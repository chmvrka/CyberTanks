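; Trigger box that shows a one-time tutorial-style pop-up when a BP_Vehicle overlaps it.
; BeginPlay checks DT_PopUpData against level name and PopUpID to pre-create the media and text widget, but breaks after the first found row, matching or not.
; Overlap displays the widget and starts a timer from the row's TimeToClose, which removes it and destroys the Blocker actor.
; The construction script applies box extent and in-game visibility.
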(event `self.ReceiveBeginPlay`
  (bind _returnvalue (`GameplayStatics.GetCurrentLevelName` true))
  (set `self.MapName` _returnvalue)
  (bind _outrownames (`DataTableFunctionLibrary.GetDataTableRowNames` "/Game/CyberTanks/MapRelatedBPs/PopUp/DT_PopUpData.DT_PopUpData"))
  (for _array_element _outrownames
    (bind _returnvalue_2 (`|GetDataTableRow` "/Game/CyberTanks/MapRelatedBPs/PopUp/DT_PopUpData.DT_PopUpData" _array_element)
      (:`then`
        (`|ExecutionSequence`
          (:`then_0`
            (bind (_video _text _time_to_close _map_name _id) (break `/Game/CyberTanks/MapRelatedBPs/PopUp/Struct_PopUp_Info` _returnvalue_2))
            (if (and (`KismetStringLibrary.EqualEqual_StrStr` _map_name (`self.MapName`)) (== _id (`self.PopUp ID`)))
              (set `self.TimeToClose` _time_to_close)
              (bind _returnvalue_3 (`|CreateWidget` "/Game/CyberTanks/MapRelatedBPs/PopUp/WBP_PopUpWidget.WBP_PopUpWidget_C" null "/Game/Movies/SoundWaveMediaplayer.SoundWaveMediaplayer" "/Game/Movies/SoundWave_Animation.SoundWave_Animation" _video _text))
              (set `self.Widget` _returnvalue_3)
              (`KismetSystemLibrary.PrintString` "Found match")))
          (:`then_1`
            (break)))))))

(event `self.CollisionToProc.OnComponentBeginOverlap`
  (params (OverlappedComponent :type "PrimitiveComponent Object Reference") (OtherActor :type "Actor Object Reference") (OtherComp :type "PrimitiveComponent Object Reference") (OtherBodyIndex :type Integer) (bFromSweep :type Boolean) (SweepResult :type "HitResult Structure (by ref)"))
  (if (not (`self.AlreadyPopped`))
    (`KismetSystemLibrary.IsObjectOfSoftClass` OtherActor "/Game/CyberTanks/TankBase/Vehicle/BP_Vehicle.BP_Vehicle_C"
      (:`True`
        (set `self.AlreadyPopped` true)
        (`UserWidget.AddToViewport` (`self.Widget`) 0)
        (`KismetSystemLibrary.K2_SetTimerDelegate` (delegate `ClosePopUp`) (`self.TimeToClose`))))))

(event `ClosePopUp`
  (`Widget.RemoveFromParent` (`self.Widget`))
  (`self.K2_DestroyActor` (`self.Blocker`)))

(fn `UserConstructionScript`
  (`BoxComponent.SetBoxExtent` (`self.CollisionToProc`) (`KismetMathLibrary.MakeVector` (`self.Box Extent X`) (`self.Box Extent Y`) (`self.Box Extent Z`)) true)
  (`SceneComponent.SetHiddenInGame` (`self.CollisionToProc`) (`self.Box Extend Hidden in Game`) false))