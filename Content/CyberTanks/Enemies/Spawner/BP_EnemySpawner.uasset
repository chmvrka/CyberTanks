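; Enemy spawner actor that places groups of melee and shooting AI enemies inside its box volume when Trigger is called.
; Trigger runs both spawn events in sequence, each looping over its own configurable count with a fixed pawn class and behavior tree.
; Each spawn picks a random point in the box bounds, projects it onto the navigation mesh, and uses the box's rotation.
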(event `Trigger`
  (`|ExecutionSequence`
    (:`then_0`
      (`self.Spawn Melee Enemy`))
    (:`then_1`
      (`self.Spawn Shooting Enemy`))))

(event `Spawn Melee Enemy`
  (bind _box (`self.Box`))
  (bind (_origin _boxextent) (`KismetSystemLibrary.GetComponentBounds` _box))
  ; Melee Spawn
  (for _ (range 1 (+ (`self.MeleeEnemyCount`) 1))
    (`AIBlueprintHelperLibrary.SpawnAIFromClass` "/Game/CyberTanks/Enemies/EnemyBases/Melee/BP_Enemy_Melee_SingleModule.BP_Enemy_Melee_SingleModule_C" "/Game/CyberTanks/Enemies/EnemyBehaviour/MeleeEnemies/BT_MeleeEnemy.BT_MeleeEnemy" (`NavigationSystemV1.K2_ProjectPointToNavigation` (`KismetMathLibrary.RandomPointInBoundingBox` _origin _boxextent) null null _boxextent) (`SceneComponent.K2_GetComponentRotation` _box) false null)))

(event `Spawn Shooting Enemy`
  (bind _box (`self.Box`))
  (bind (_origin _boxextent) (`KismetSystemLibrary.GetComponentBounds` _box))
  ; Shooting Spawn
  (for _ (range 1 (+ (`self.ShootingEnemyCount`) 1))
    (`AIBlueprintHelperLibrary.SpawnAIFromClass` "/Game/CyberTanks/Enemies/EnemyBases/Ranged/BP_Enemy_Moving_Base.BP_Enemy_Moving_Base_C" "/Game/CyberTanks/Enemies/EnemyBehaviour/ShootingEnemies/BT_ShootingEnemy.BT_ShootingEnemy" (`NavigationSystemV1.K2_ProjectPointToNavigation` (`KismetMathLibrary.RandomPointInBoundingBox` _origin _boxextent) null null _boxextent) (`SceneComponent.K2_GetComponentRotation` _box) false null)))

(fn `UserConstructionScript`)