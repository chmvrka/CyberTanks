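; Base saw blade for melee enemies in CyberTanks that damages the health and energy of actors touching it.
; A timeline started on BeginPlay animates the saw mesh's pitch.
; When an actor implementing BPI_Energon enters the box, it is stored and a looping timer starts sending it damage messages through RepeatedDamage.
; Leaving the box clears the overlap flag and the timer.
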(event `self.ReceiveBeginPlay`
  (bind (_direction _newtrack_0) (`Timeline|Rotator`)
    (:`Update`
      (`SceneComponent.K2_SetRelativeRotation` (`self.Saw`) (`KismetMathLibrary.MakeRotator` 0.0 _newtrack_0) false false))))

(event `self.Box.OnComponentBeginOverlap`
  (params (OverlappedComponent :type "PrimitiveComponent Object Reference") (OtherActor :type "Actor Object Reference") (OtherComp :type "PrimitiveComponent Object Reference") (OtherBodyIndex :type Integer) (bFromSweep :type Boolean) (SweepResult :type "HitResult Structure (by ref)"))
  (if (`KismetSystemLibrary.DoesImplementInterface` OtherActor "/Game/CyberTanks/EnergonComponent/BPI_Energon.BPI_Energon_C")
    (set `self.Player` OtherActor)
    (set `self.Overlaping?` true)
    (bind _returnvalue (`KismetSystemLibrary.K2_SetTimer` null "RepeatedDamage" 0.7 true))
    (set `self.Timer` _returnvalue)))

(event `self.Box.OnComponentEndOverlap`
  (params (OverlappedComponent :type "PrimitiveComponent Object Reference") (OtherActor :type "Actor Object Reference") (OtherComp :type "PrimitiveComponent Object Reference") (OtherBodyIndex :type Integer))
  (if (`KismetSystemLibrary.DoesImplementInterface` OtherActor "/Game/CyberTanks/EnergonComponent/BPI_Energon.BPI_Energon_C")
    (set `self.Overlaping?` false)
    (`KismetSystemLibrary.K2_ClearAndInvalidateTimerHandle` (`self.Timer`))))

(fn `RepeatedDamage`
  (if (`self.Overlaping?`)
    (message `/Game/CyberTanks/EnergonComponent/BPI_Energon.Damage` (`self.Player`) (`self.HPDamage`) (`self.EnergyDamage`))))

(fn `UserConstructionScript`)