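; Base ranged enemy pawn that spots the player vehicle, turns to face it and fires bullets until it loses sight.
; PawnSensing stores the tagged player and unpauses a looping timer that spawns BP_Bullet at the Arrow.
; Tick aims the PoseableMesh at the player and pauses that timer about two seconds after the last sighting.
; Damage drains HP and Energy, destroying the pawn when HP runs out; TurretAttack is empty.
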(event `self.ReceiveBeginPlay`
  ;[0.5469 0.03959 0.05591 0.5] BeginPlay
  (bind _returnvalue (`KismetSystemLibrary.K2_SetTimerDelegate` (delegate `Shoot`) (`self.AtackTimeDelay`) true))
  (bind _output_get (set `self.AttackEventTimer` _returnvalue))
  (`KismetSystemLibrary.K2_PauseTimerHandle` _output_get))

(event `self.ReceiveTick`
  (params (DeltaSeconds :type "Float (single-precision)"))
  ;[0.5938 0.04467 0 0.5] EVENT TICK
  (bind _player (`self.player`)
    (:`then`
      (if (`self.IsPlayerVisible`)
        (`SceneComponent.K2_SetWorldRotation` (`self.PoseableMesh`) (`KismetMathLibrary.Conv_VectorToRotator` (- (`self.K2_GetActorLocation` _player) (`SceneComponent.K2_GetComponentLocation` (`self.PoseableMesh`)))) false false)
        (if (> (- (`GameplayStatics.GetTimeSeconds`) (`self.LastSeenTime`)) 2.0)
          (set `self.IsPlayerVisible` false)
          (`KismetSystemLibrary.K2_PauseTimerHandle` (`self.AttackEventTimer`)))))
    (:`else`)))

(event `self.PawnSensing.OnSeePawn`
  (params (Pawn :type "Pawn Object Reference"))
  ;[0.2565 0.4792 0.1073 0.5] OnSee
  (set `self.LastSeenTime` (`GameplayStatics.GetTimeSeconds`))
  (if (`self.ActorHasTag` Pawn "PlayerVehicle")
    (set `self.IsPlayerVisible` true)
    (set `self.player` Pawn)
    (`KismetSystemLibrary.K2_UnPauseTimerHandle` (`self.AttackEventTimer`))))

(event `Shoot`
  (bind _arrow (`self.Arrow`))
  ;[0.15 0.1148 0.02618 0.5] ShootEvent
  (`|SpawnActorFromClass` "/Game/CyberTanks/TankBase/Modules/CannonModule/BP_Bullet.BP_Bullet_C" (`KismetMathLibrary.MakeTransform` (`SceneComponent.K2_GetComponentLocation` _arrow) (`SceneComponent.K2_GetComponentRotation` _arrow)) "AdjustIfPossibleButAlwaysSpawn" "MultiplyWithRoot" null 5.0 5.0 1500.0 null))

(event `/Game/CyberTanks/EnergonComponent/BPI_Energon.Damage`
  (params (HPDamage :type "Float (double-precision)") (EnergyDamage :type "Float (double-precision)"))
  (set `self.HP` (- (`self.HP`) HPDamage))
  (set `self.Energy` (- (`self.Energy`) EnergyDamage))
  (if (<= (`self.HP`) 0.0)
    (`KismetSystemLibrary.PrintString` "Kill Logic")
    (`self.K2_DestroyActor`)))

(event `self.ReceiveEndPlay`
  (params (EndPlayReason :type "EEndPlayReason Enum" :default "Destroyed")))

(fn `TurretAttack`)

(fn `UserConstructionScript`)