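; Base character for moving ranged enemies in CyberTanks, with a weapon module, HP and Energy.
; On BeginPlay it spawns its offensive class and attaches it to the WeaponModule mesh socket.
; Pawn sensing writes any PlayerVehicle-tagged pawn to the AI blackboard as spotted.
; Depleted Energy temporarily disables movement, while depleted HP destroys the enemy and its weapon with an explosion effect and sound.
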(event `self.ReceiveDestroyed`
  (bind _returnvalue (`self.K2_GetActorLocation`))
  ; Spawn
  (`GameplayStatics.SpawnEmitterAtLocation` "/Game/StarterContent/Particles/P_Explosion.P_Explosion" _returnvalue (struct) (10.0 10.0 10.0))
  (`self.K2_DestroyActor` (stale `self.ReceiveBeginPlay` _returnvalue))
  (`GameplayStatics.PlaySoundAtLocation` "/Game/StarterContent/Audio/Explosion02.Explosion02" _returnvalue (struct) 1.0 1.0 0.0 null null null null))

(event `OnDestroyed_Event` :!signature `self.OnDestroyed`
  (params (DestroyedActor :type "Actor Object Reference"))
  ; Spawn
)

(event `/Game/CyberTanks/EnergonComponent/BPI_Energon.Damage`
  (params (HPDamage :type "Float (double-precision)") (EnergyDamage :type "Float (double-precision)"))
  (bind _charactermovement (`self.CharacterMovement`))
  (set `self.HP` (- (`self.HP`) HPDamage))
  (set `self.Energy` (- (`self.Energy`) EnergyDamage))
  (`|ExecutionSequence`
    (:`then_0`
      (if (<= (`self.Energy`) 0.0)
        (`CharacterMovementComponent.SetMovementMode` _charactermovement "MOVE_None" 0)
        (`KismetSystemLibrary.Delay` 4.0)
        (`CharacterMovementComponent.SetMovementMode` _charactermovement "MOVE_Walking" 0)))
    (:`then_1`
      (if (<= (`self.HP`) 0.0)
        (`KismetSystemLibrary.PrintString` "Kill Logic")
        (`self.K2_DestroyActor`)))))

(event `self.ReceiveBeginPlay`
  (bind (_returnvalue_location _returnvalue_rotation) (`KismetMathLibrary.BreakTransform` (`SceneComponent.GetSocketTransform` (`self.Mesh`) "WeaponModule" "RTS_World")))
  ; Spawn
  (bind _returnvalue (`|SpawnActorFromClass` (`self.OffensiveClassSpawn`) (`KismetMathLibrary.MakeTransform` _returnvalue_location _returnvalue_rotation) "AlwaysSpawn" "MultiplyWithRoot" null null))
  (add `self.OnDestroyed` (delegate `OnDestroyed_Event`))
  (`self.K2_AttachToComponent` _returnvalue (`self.Mesh`) "WeaponModule" "KeepWorld" "KeepWorld" "KeepRelative" true))

(event `self.PawnSensing.OnSeePawn`
  (params (Pawn :type "Pawn Object Reference"))
  (bind _returnvalue (`AIBlueprintHelperLibrary.GetBlackboard` (`AIBlueprintHelperLibrary.GetAIController` self)))
  ;[0.1388 1 0 0.5] OnSeePawn
  (set `self.LastSeenTime` (`GameplayStatics.GetTimeSeconds`))
  (if (`self.ActorHasTag` Pawn "PlayerVehicle")
    (`BlackboardComponent.SetValueAsObject` _returnvalue "PlayerVehicle" Pawn)
    (`BlackboardComponent.SetValueAsBool` _returnvalue "playerSpotted?" true)))

(fn `UserConstructionScript`)