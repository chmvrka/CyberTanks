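; Energon actor component for CyberTanks that tracks HP and energy and derives an operational, repair, recharge or disabled state from them.
; Damage lowers both pools unless invulnerable, then re-evaluates state and fires dispatchers when HP, energy or both are depleted.
; Bound restore dispatchers refill either or both pools, to half when a part is carried, with optional timed invulnerability that ends in a state recheck.
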(event `FullRestore_Event` :!signature `self.FullRestore`
  (params (WithInvoulnerability :type Boolean) (`PartCarried?` :type Boolean))
  ; Full heal events
  (`self.FullRestoreHp` false `PartCarried?`)
  (`self.FullRestoreEnergy` WithInvoulnerability `PartCarried?`)
  (`self.HpOrEnergyChanged` :!label _label))

(event `FullRestoreHp_Event` :!signature `self.FullRestoreHp`
  (params (WithInvulnerability :type Boolean) (`PartCarried?` :type Boolean))
  ; Full heal events
  (if WithInvulnerability
    (`self.InvulnerableState`))
  (if (not `PartCarried?`)
    (set `self.HP` (`self.MaxHp`))
    (goto _label)
    (else
      (set `self.HP` (* (`self.MaxHp`) 0.5))
      (goto _label))))

(event `FullRestoreEnergy_Event` :!signature `self.FullRestoreEnergy`
  (params (WithInvulnerability :type Boolean) (`PartCarried?` :type Boolean))
  ; Full heal events
  (if WithInvulnerability
    (`self.InvulnerableState`))
  (if (not `PartCarried?`)
    (set `self.Energy` (`self.MaxEnergy`))
    (goto _label)
    (else
      (set `self.Energy` (* (`self.MaxEnergy`) 0.5))
      (goto _label))))

(event `self.ReceiveBeginPlay`
  ;[0 1 0 0.5] BeginPlay
  (`self.FullRestore` false)
  ; Full heal events
  (add `self.FullRestore` (`|CreateDelegate` :!event `FullRestore_Event`))
  (add `self.FullRestoreHp` (`|CreateDelegate` :!event `FullRestoreHp_Event`))
  (add `self.FullRestoreEnergy` (`|CreateDelegate` :!event `FullRestoreEnergy_Event`)))

(event `Damage`
  (params (HP :type "Float (double-precision)") (Energy :type "Float (double-precision)"))
  ; Damage and CheckState
  (if (`|EnumInequality` (`self.EnergonState`) "NewEnumerator0")
    (set `self.HP` (- (`self.HP`) HP))
    (set `self.Energy` (- (`self.Energy`) Energy))
    (`self.CheckState`)
    (`self.HpOrEnergyChanged`)))

(event `CheckState`
  ; Damage and CheckState
  (bind _energonstate (`self.EnergonStateF`))
  (switch `/Game/CyberTanks/EnergonComponent/ENUM_EnergonState` _energonstate
    (:`NewEnumerator2`
      (`self.HPZero`))
    (:`NewEnumerator3`
      (`self.EnergyZero`))
    (:`NewEnumerator4`
      (`self.HPAndEnergyZero`))))

(event `InvulnerableState`
  ; Invulnerability
  (set `self.EnergonState` "NewEnumerator0")
  (`KismetSystemLibrary.K2_SetTimerDelegate` (`|CreateDelegate` :!event `VulnerableAgain`) (`self.InvulnerableTime`)))

(event `VulnerableAgain`
  ; Invulnerability
  (set `self.EnergonState` "NewEnumerator5")
  (`self.CheckState`))

(fn `EnergonStateF`
  (returns (EnergonState :type "/Game/CyberTanks/EnergonComponent/ENUM_EnergonState Enum"))
  (bind _energystate (`self.EnergyStateF`))
  (bind _hpstate (`self.HPStateF`))
  (switch `/Game/CyberTanks/EnergonComponent/ENUM_HPState` _hpstate
    (:`NewEnumerator0`
      (switch `/Game/CyberTanks/EnergonComponent/ENUM_EnergyState` _energystate
        (:`NewEnumerator1`
          (set `self.EnergonState` "NewEnumerator1" :!label _label))
        (:`NewEnumerator2`
          (goto _label))
        (:`NewEnumerator3`
          (set `self.EnergonState` "NewEnumerator3" :!label _label_2))))
    (:`NewEnumerator1`
      (switch `/Game/CyberTanks/EnergonComponent/ENUM_EnergyState` _energystate
        (:`NewEnumerator1`
          (goto _label))
        (:`NewEnumerator2`
          (goto _label))
        (:`NewEnumerator3`
          (goto _label_2))))
    (:`NewEnumerator2`
      (switch `/Game/CyberTanks/EnergonComponent/ENUM_EnergyState` _energystate
        (:`NewEnumerator1`
          (set `self.EnergonState` "NewEnumerator2" :!label _label_3))
        (:`NewEnumerator2`
          (goto _label_3))
        (:`NewEnumerator3`
          (set `self.EnergonState` "NewEnumerator4")))))
  (return (`self.EnergonState`)))

(fn `EnergyStateF`
  (returns (EnergyState :type "/Game/CyberTanks/EnergonComponent/ENUM_EnergyState Enum"))
  (if (<= (`self.Energy`) 0.0)
    (bind _output_get (set `self.EnergyState` "NewEnumerator3"))
    (return _output_get)
    (elif (< (`self.Energy`) (`self.MaxEnergy`))
      (bind _output_get_2 (set `self.EnergyState` "NewEnumerator2"))
      (return _output_get_2)
      (elif (== (`self.Energy`) (`self.MaxEnergy`))
        (bind _output_get_3 (set `self.EnergyState` "NewEnumerator1"))
        (return _output_get_3)))))

(fn `HPStateF`
  (returns (HPState :type "/Game/CyberTanks/EnergonComponent/ENUM_HPState Enum"))
  (if (<= (`self.HP`) 0.0)
    (bind _output_get (set `self.HPState` "NewEnumerator2"))
    (return _output_get)
    (elif (< (`self.HP`) (`self.MaxHp`))
      (bind _output_get_2 (set `self.HPState` "NewEnumerator1"))
      (return _output_get_2)
      (elif (== (`self.HP`) (`self.MaxHp`))
        (bind _output_get_3 (set `self.HPState` "NewEnumerator0"))
        (return _output_get_3)))))