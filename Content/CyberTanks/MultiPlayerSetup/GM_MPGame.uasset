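; Game mode for local multiplayer CyberTanks levels, where player characters share one modular tank.
; On BeginPlay it creates three extra local players, assigns each controller an index and minigame render target, and shows the level's data-table briefing.
; Outside TankConfiguration, it spawns the saved tank at the vehicle spawn point and moves all characters onto it.
; SaveAndBuildNewTank builds a replacement, moves players over, saves the configuration and destroys other tanks.
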(event `self.ReceiveBeginPlay`
  (`|ExecutionSequence`
    (:`then_0`
      ; GameMode Init
      (`self.InitPlayers`)
      (bind _asbp_mpgame_instance (cast `/Game/CyberTanks/MultiPlayerSetup/BP_MPGameInstance` (`GameplayStatics.GetGameInstance`)))
      (if (`/Game/CyberTanks/MultiPlayerSetup/BP_MPGameInstance.SaveLoaded` _asbp_mpgame_instance)
        (bind _returnvalue (`GameplayStatics.GetCurrentLevelName` true))
        (if (not (`KismetStringLibrary.EqualEqual_StrStr` _returnvalue "TankConfiguration"))
          (bind _save_game (`/Game/CyberTanks/MultiPlayerSetup/BP_MPGameInstance.Save Game` _asbp_mpgame_instance))
          (`self.BuildTank` (`/Game/CyberTanks/MultiPlayerSetup/BP_SaveGame.ModuleNames` _save_game) (`/Game/CyberTanks/MultiPlayerSetup/BP_SaveGame.VehicleBaseName` _save_game))
          (`self.TransportPlayersToNewTank`))
        (else
          (`KismetSystemLibrary.PrintString` "GM_MPGame Save NOT loaded !!!!!!!!!!!!!!!!!!!!!!!!!!!!!!!!!!!!!!!!!!!!!!!!!!!!!!!!!!!!!!!!!!!!!!!!!!!!!!!!!!!!!!!!!!!!!!!!!!!!!!!!!!!!!!!!!!!!!!!!!!!!!!!!!!!!!!!!!!!!!!!!" true true (struct :`R` 1.0 :`G` 0.012221 :`A` 1.0) 100000.0 "-1"))))
    (:`then_1`
      (bind _returnvalue_2 (`GameplayStatics.GetCurrentLevelName` true))
      (bind _returnvalue_3 (`|GetDataTableRow` "/Game/CyberTanks/UI/LoadingScreens/DT_WidgetInfoBriefing.DT_WidgetInfoBriefing" (`KismetStringLibrary.Conv_StringToName` _returnvalue_2))
        (:`then`
          (bind (_image _mapname _lore _imagemaybe _drugastrona) (break `/Game/CyberTanks/UI/LoadingScreens/STRUCT_LoadingScreenWidget` _returnvalue_3))
          (bind _returnvalue_4 (`|CreateWidget` "/Game/CyberTanks/UI/LoadingScreens/WBP_BriefingScreen.WBP_BriefingScreen_C" null _image _mapname _lore _imagemaybe _drugastrona))
          (`UserWidget.AddToViewport` _returnvalue_4 0))))))

(event `InitPlayers`
  ; Players INIT
  (bind _returnvalue (`GameplayStatics.GetActorOfClass` "/Game/CyberTanks/MultiPlayerSetup/PC_MPGame.PC_MPGame_C"))
  (`/Engine/EditorBlueprintResources/StandardMacros.IsValid` _returnvalue
    (:`Is Valid`
      (`KismetArrayLibrary.Array_AddUnique` (`self.PlayerControllers`) _returnvalue)
      (for _ (range 1 4)
        (bind _returnvalue_2 (`GameplayStatics.CreatePlayer` -1))
        (bind _aspc_mpgame (cast `/Game/CyberTanks/MultiPlayerSetup/PC_MPGame` _returnvalue_2))
        (`KismetArrayLibrary.Array_AddUnique` (`self.PlayerControllers`) _aspc_mpgame))
      (set `self.DefaultPawnClass` "/Game/ThirdPerson/Blueprints/BP_ThirdPersonCharacter.BP_ThirdPersonCharacter_C")
      ;; Assigning render targets for minigames to each controller
      (bind _outactors (`GameplayStatics.GetAllActorsOfClass` "/Game/CyberTanks/MultiPlayerSetup/PC_MPGame.PC_MPGame_C"))
      (for (_array_element _array_index) _outactors
        (set `/Game/CyberTanks/MultiPlayerSetup/PC_MPGame.RenderTarget` (`|GetArrayItem` (`self.RenderTexturesForMiniGames`) _array_index) _array_element)
        (set `/Game/CyberTanks/MultiPlayerSetup/PC_MPGame.RenderMaterial` (`|GetArrayItem` (`self.MaterialForRT`) _array_index) _array_element)
        (set `/Game/CyberTanks/MultiPlayerSetup/PC_MPGame.PlayerIndex` _array_index _array_element))
      ;; W teorii ma zniknac myszka
      (`KismetSystemLibrary.DelayUntilNextTick`)
      (set `PlayerController.bShowMouseCursor` false (`GameplayStatics.GetPlayerController` 0)))))

(event `SaveAndBuildNewTank`
  (params (Modules :type "Array of /Game/CyberTanks/TankConfiguration/ENUM_ModuleNames Enum") (VehicleBase :type "/Game/CyberTanks/TankConfiguration/ENUM_VehicleBaseNames Enum" :default "NewEnumerator0"))
  ; Spawn Tank and Save
  (`self.BuildTank` Modules VehicleBase)
  (`self.TransportPlayersToNewTank`)
  (bind _asbp_mpgame_instance (cast `/Game/CyberTanks/MultiPlayerSetup/BP_MPGameInstance` (`GameplayStatics.GetGameInstance`)))
  (`/Game/CyberTanks/MultiPlayerSetup/BP_MPGameInstance.ModifySaveFile` _asbp_mpgame_instance Modules VehicleBase "NewEnumerator6" "NewEnumerator5" "None")
  (`self.DeleteOldTank`))

(event `TestPrint`
  (params (`module names` :type "Array of /Game/CyberTanks/TankConfiguration/ENUM_ModuleNames Enum") (`vehicle name` :type "/Game/CyberTanks/TankConfiguration/ENUM_VehicleBaseNames Enum" :default "NewEnumerator0"))
  ; Test print
  (for _array_element `module names`
    (set `self.TestStringVar` (`KismetStringLibrary.Concat_StrStr` (`self.TestStringVar`) (`|GetEnumeratorNameAsString` _array_element) " \n")))
  (`KismetSystemLibrary.PrintText` (`|FormatText` "Config to save: \nnunmber of parts:{a} \nvehicle base:{b} \npart names: \n{c}" (`KismetArrayLibrary.Array_Length` `module names`) (`|GetEnumeratorNameAsString` `vehicle name`) (`|FormatText` (`KismetTextLibrary.Conv_StringToText` (`self.TestStringVar`)))) true true (struct :`G` 1.0 :`B` 0.663957 :`A` 1.0) 20.0))

(event `TransportPlayersToNewTank`
  ; Transport playters to Tank
  (bind _outactors (`GameplayStatics.GetAllActorsOfClass` "/Game/ThirdPerson/Blueprints/BP_ThirdPersonCharacter.BP_ThirdPersonCharacter_C"))
  (for _array_element _outactors
    (`self.TransportSpecificPlayerToTank` _array_element)))

(event `BuildTank`
  (params (Modules :type "Array of /Game/CyberTanks/TankConfiguration/ENUM_ModuleNames Enum") (VehicleBase :type "/Game/CyberTanks/TankConfiguration/ENUM_VehicleBaseNames Enum" :default "NewEnumerator0"))
  ; Spawn Tank
  (bind _returnvalue (`|GetDataTableRow` "/Game/CyberTanks/TankConfiguration/DT_TankBaseList.DT_TankBaseList" (`KismetStringLibrary.Conv_StringToName` (`|GetEnumeratorNameAsString` VehicleBase)))
    (:`then`
      (bind _returnvalue_2 (`GameplayStatics.GetActorOfClass` "/Game/CyberTanks/MapRelatedBPs/BP_VehicleSpawnPoint.BP_VehicleSpawnPoint_C"))
      (`/Engine/EditorBlueprintResources/StandardMacros.IsValid` _returnvalue_2
        (:`Is Valid`
          (bind _returnvalue_3 (`|SpawnActorFromClass` (`.Base_5_5EA3261E469403E43662BFBD74D85AC1` (break `/Game/CyberTanks/TankConfiguration/STRUCT_TankBase` _returnvalue)) (`self.GetTransform` _returnvalue_2) "AlwaysSpawn" "MultiplyWithRoot" null Modules (break `/Game/CyberTanks/TankConfiguration/STRUCT_TankBase` _returnvalue) null))
          ;;[0.15 0 0.01484 0.5] Test if not needed and YEET OUT
          (bind _asbp_mpgame_instance (cast `/Game/CyberTanks/MultiPlayerSetup/BP_MPGameInstance` (`GameplayStatics.GetGameInstance`)))
          (set `/Game/CyberTanks/MultiPlayerSetup/BP_MPGameInstance.Tank` _returnvalue_3 _asbp_mpgame_instance)
          (set `self.CurrentOneAndOnlyTank` _returnvalue_3))
        (:`Is Not Valid`
          (`KismetSystemLibrary.PrintString` "I dont know how to fix that GM_MPGame"))))))

(event `TransportSpecificPlayerToTank`
  (params (PlayerChar :type "/Game/ThirdPerson/Blueprints/BP_ThirdPersonCharacter Object Reference"))
  (bind _currentoneandonlytank (`self.CurrentOneAndOnlyTank`))
  ; Transport playters to Tank
  (`self.RestartPlayer` (`Pawn.GetController` PlayerChar))
  (set `/Game/ThirdPerson/Blueprints/BP_ThirdPersonCharacter.Floor` _currentoneandonlytank PlayerChar)
  (`self.K2_SetActorLocation` PlayerChar (`SceneComponent.K2_GetComponentLocation` (`/Game/CyberTanks/TankBase/Vehicle/BP_Vehicle.SpawnPoint` _currentoneandonlytank)) false false))

(event `DeleteOldTank`
  ; Delete Tank that should not be there
  (bind _outactors (`GameplayStatics.GetAllActorsOfClass` "/Game/CyberTanks/TankBase/Vehicle/BP_Vehicle.BP_Vehicle_C"))
  (`KismetArrayLibrary.Array_RemoveItem` _outactors (`self.CurrentOneAndOnlyTank`))
  (`self.K2_DestroyActor` _outactors))

(fn `MotherFuckingGiveMePC`
  (params (ID :type Integer))
  (returns (Controller :type "/Game/CyberTanks/MultiPlayerSetup/PC_MPGame Object Reference"))
  (locals (ReturnPC :type "/Game/CyberTanks/MultiPlayerSetup/PC_MPGame Object Reference"))
  (for _array_element (`self.PlayerControllers`)
    (if (== (`/Game/CyberTanks/MultiPlayerSetup/PC_MPGame.PlayerIndex` _array_element) ID)
      (bind _output_get (set `local.ReturnPC` _array_element))
      (`KismetSystemLibrary.PrintString` (`KismetSystemLibrary.GetDisplayName` _output_get) true true (struct :`R` 1.0 :`B` 0.119016 :`A` 1.0))))
  (return (`local.ReturnPC`)))

(fn `UserConstructionScript`)