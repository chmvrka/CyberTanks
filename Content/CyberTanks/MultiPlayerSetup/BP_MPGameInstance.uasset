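; Game instance for CyberTanks multiplayer setup that owns the persistent save of tank loadout, unlocks and beaten maps.
; Init async-loads the "test" slot, creating a default save and retrying if missing, then clears map progress for testing.
; ModifySaveFile updates the cached save, skipping empty or sentinel inputs and adding unlocks uniquely, then writes to disk.
; SaveGame writes a fresh save object, preferring the current Tank's loadout over the cached one.
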(event `PrintTestTankVar`
  (bind _tank (`self.Tank`))
  (bind _modulenames (`/Game/CyberTanks/TankBase/Vehicle/BP_Vehicle.ModuleNames` _tank))
  ; Test print tank var
  (`/Engine/EditorBlueprintResources/StandardMacros.IsValid` _tank
    (:`Is Valid`
      (for _array_element _modulenames
        (set `self.SaveTestVarForPrintTest` (`KismetStringLibrary.Concat_StrStr` (`self.SaveTestVarForPrintTest`) (`|GetEnumeratorNameAsString` _array_element) " \n")))
      (`KismetSystemLibrary.PrintText` (`|FormatText` "Saving Tank: \nnunmber of parts:{a} \nvehicle base:{b} \npart names: \n{c}" (`KismetArrayLibrary.Array_Length` _modulenames) (`|GetEnumeratorNameAsString` (`/Game/CyberTanks/TankBase/Vehicle/BP_Vehicle.VehicleBaseName` _tank)) (`|FormatText` (`KismetTextLibrary.Conv_StringToText` (`self.SaveTestVarForPrintTest`)))) true true (struct :`G` 1.0 :`B` 0.663957 :`A` 1.0) 20.0))
    (:`Is Not Valid`
      (`KismetSystemLibrary.PrintString` "BP_MPGameInstance, tank var not valid in test print tank var" true true (struct :`R` 1.0 :`G` 0.636384 :`A` 1.0) 20.0))))

(event `RestartInit`
  (bind _returnvalue (`GameplayStatics.DoesSaveGameExist` "test" :!label _label))
  (if _returnvalue
    (bind _savegame (`AsyncActionHandleSaveGame.AsyncLoadGameFromSlot` "test")
      (:`Completed`
        (set `self.SaveLoaded` true)
        (bind _asbp_save_game (cast `/Game/CyberTanks/MultiPlayerSetup/BP_SaveGame` _savegame))
        (bind _output_get (set `self.Save Game` _asbp_save_game))
        ; Each game start clears map progress(leave for testing)
        (`KismetArrayLibrary.Array_Clear` (`/Game/CyberTanks/MultiPlayerSetup/BP_SaveGame.MapsPlayed` _output_get))
        (`self.SaveSaveFileToDisk` "test")))
    (else
      ; If no save file found
      (`self.CreateDefaultSave`)
      (`self.RestartInit`))))

(event `self.ReceiveInit`
  ;[0 1 0.1 0.5] START
  (goto _label))

(event `SaveGame`
  (bind _save_game (`self.Save Game`))
  (bind _save_game_2 (`self.Save Game`))
  (bind _tank (`self.Tank`))
  ; create object of savegame, that with tank setup
  (bind _returnvalue (`GameplayStatics.CreateSaveGameObject` "/Game/CyberTanks/MultiPlayerSetup/BP_SaveGame.BP_SaveGame_C"))
  (`/Engine/EditorBlueprintResources/StandardMacros.IsValid` _tank
    (:`Is Valid`
      (set `/Game/CyberTanks/MultiPlayerSetup/BP_SaveGame.ModuleNames` (`/Game/CyberTanks/TankBase/Vehicle/BP_Vehicle.ModuleNames` _tank) _returnvalue)
      (set `/Game/CyberTanks/MultiPlayerSetup/BP_SaveGame.VehicleBaseName` (`/Game/CyberTanks/TankBase/Vehicle/BP_Vehicle.VehicleBaseName` _tank) _returnvalue)
      (set `/Game/CyberTanks/MultiPlayerSetup/BP_SaveGame.Unlocks` (`/Game/CyberTanks/MultiPlayerSetup/BP_SaveGame.Unlocks` _save_game_2) _returnvalue)
      (set `/Game/CyberTanks/MultiPlayerSetup/BP_SaveGame.MapsPlayed` (`/Game/CyberTanks/MultiPlayerSetup/BP_SaveGame.MapsPlayed` _save_game_2) _returnvalue)
      ; making save file on disk
      (`GameplayStatics.SaveGameToSlot` _returnvalue "test"))
    (:`Is Not Valid`
      (set `/Game/CyberTanks/MultiPlayerSetup/BP_SaveGame.ModuleNames` (`/Game/CyberTanks/MultiPlayerSetup/BP_SaveGame.ModuleNames` _save_game) _returnvalue)
      (set `/Game/CyberTanks/MultiPlayerSetup/BP_SaveGame.VehicleBaseName` (`/Game/CyberTanks/MultiPlayerSetup/BP_SaveGame.VehicleBaseName` _save_game) _returnvalue)
      (set `/Game/CyberTanks/MultiPlayerSetup/BP_SaveGame.Unlocks` (`/Game/CyberTanks/MultiPlayerSetup/BP_SaveGame.Unlocks` _save_game) _returnvalue)
      (set `/Game/CyberTanks/MultiPlayerSetup/BP_SaveGame.MapsPlayed` (`/Game/CyberTanks/MultiPlayerSetup/BP_SaveGame.MapsPlayed` _save_game) _returnvalue)
      (`GameplayStatics.SaveGameToSlot` _returnvalue "test"))))

(event `CreateDefaultSave`
  ; Default Save, here should be setup for first tank for first map, here is no checking so test it out if its working
  (bind _returnvalue (`GameplayStatics.CreateSaveGameObject` "/Game/CyberTanks/MultiPlayerSetup/BP_SaveGame.BP_SaveGame_C"))
  (set `/Game/CyberTanks/MultiPlayerSetup/BP_SaveGame.ModuleNames` (`|MakeArray` "NewEnumerator0" "NewEnumerator1" "NewEnumerator2" :!type "/Game/CyberTanks/TankConfiguration/ENUM_ModuleNames Enum") _returnvalue)
  (set `/Game/CyberTanks/MultiPlayerSetup/BP_SaveGame.VehicleBaseName` "NewEnumerator0" _returnvalue)
  (`GameplayStatics.SaveGameToSlot` _returnvalue "test"))

(fn `ModifySaveFile`
  (params (TankModuleNames :type "Array of /Game/CyberTanks/TankConfiguration/ENUM_ModuleNames Enum") (TankVehicleBaseName :type "/Game/CyberTanks/TankConfiguration/ENUM_VehicleBaseNames Enum" :default "NewEnumerator5") (UnlockModuleNames :type "/Game/CyberTanks/TankConfiguration/ENUM_ModuleNames Enum" :default "NewEnumerator6") (UnlockVehicleBaseName :type "/Game/CyberTanks/TankConfiguration/ENUM_VehicleBaseNames Enum" :default "NewEnumerator5") (BeatenMapName :type Name :default "None"))
  (locals (LocalModuleNames :type "Array of /Game/CyberTanks/TankConfiguration/ENUM_ModuleNames Enum") (LocalVehicleBaseNames :type "Array of /Game/CyberTanks/TankConfiguration/ENUM_VehicleBaseNames Enum"))
  (bind _tankmodulenames (`local.TankModuleNames`))
  (bind _tankvehiclebasename (`local.TankVehicleBaseName`))
  (bind _unlockmodulenames (`local.UnlockModuleNames`))
  (bind _unlockvehiclebasename (`local.UnlockVehicleBaseName`))
  (bind (_unlockedmodules _unlockedvehicles) (break `/Game/CyberTanks/MultiPlayerSetup/Save/STRUCT_Save_UnlocksList` (`/Game/CyberTanks/MultiPlayerSetup/BP_SaveGame.Unlocks` (`self.Save Game`))))
  (bind (_unlockedmodules_2 _unlockedvehicles_2) (break `/Game/CyberTanks/MultiPlayerSetup/Save/STRUCT_Save_UnlocksList` (`/Game/CyberTanks/MultiPlayerSetup/BP_SaveGame.Unlocks` (`self.Save Game`))))
  (`/Engine/EditorBlueprintResources/StandardMacros.IsValid` (`self.Save Game`)
    (:`Is Valid`
      (`|ExecutionSequence`
        (:`then_0`
          ; Set current modules
          (if (`KismetArrayLibrary.Array_IsNotEmpty` _tankmodulenames)
            (set `/Game/CyberTanks/MultiPlayerSetup/BP_SaveGame.ModuleNames` _tankmodulenames (`self.Save Game`))))
        (:`then_1`
          ; Save current vehicle base
          (if (`|EnumInequality` _tankvehiclebasename "NewEnumerator5")
            (set `/Game/CyberTanks/MultiPlayerSetup/BP_SaveGame.VehicleBaseName` _tankvehiclebasename (`self.Save Game`))))
        (:`then_2`
          ; Add new module and vehicle unlocks
          (switch `string` (`|GetEnumeratorNameAsString` _unlockmodulenames)
            (:`Default`
              (bind _output_get (set `local.LocalModuleNames` _unlockedmodules_2))
              (`KismetArrayLibrary.Array_AddUnique` _output_get _unlockmodulenames)
              (set `/Game/CyberTanks/MultiPlayerSetup/BP_SaveGame.Unlocks` (make `/Game/CyberTanks/MultiPlayerSetup/Save/STRUCT_Save_UnlocksList` _output_get _unlockedvehicles_2) (`self.Save Game`)))
            (:`Nothing`
              _))
          (switch `string` (`|GetEnumeratorNameAsString` _unlockvehiclebasename)
            (:`Default`
              (bind _output_get_2 (set `local.LocalVehicleBaseNames` _unlockedvehicles))
              (`KismetArrayLibrary.Array_AddUnique` _output_get_2 _unlockvehiclebasename)
              (set `/Game/CyberTanks/MultiPlayerSetup/BP_SaveGame.Unlocks` (make `/Game/CyberTanks/MultiPlayerSetup/Save/STRUCT_Save_UnlocksList` _unlockedmodules _output_get_2) (`self.Save Game`)))
            (:`Nothing`)))
        (:`then_3`
          ; Add Beaten map to save
          (if (!= (`local.BeatenMapName`) "None")
            (`KismetArrayLibrary.Array_AddUnique` (`/Game/CyberTanks/MultiPlayerSetup/BP_SaveGame.MapsPlayed` (`self.Save Game`)) (`local.BeatenMapName`))))
        (:`then_4`
          (`self.SaveSaveFileToDisk` "test"))))
    (:`Is Not Valid`
      (`KismetSystemLibrary.PrintString` "SaveGame NOT valid in Game Instance" true true (struct :`R` 1.0 :`B` 0.035408 :`A` 1.0) 10000.0 "0"))))

(fn `SaveSaveFileToDisk`
  (params (SlotName :type String))
  (`GameplayStatics.SaveGameToSlot` (`self.Save Game`) SlotName))